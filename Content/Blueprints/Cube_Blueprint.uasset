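; Interactable note pickup that shows a Note_widget on screen when the player presses E while overlapping it.
; Overlap enables input and caches the PCMorningStar character; a FlipFlop on E alternates opening and closing the widget.
; Closing removes the widget, waits briefly, destroys the actor and increments the character's ImageIndex.
; Ending overlap disables input and runs that same close path, even if the note was never opened.
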(event `Key|E`
  (params (Key :type "Key Structure" :default "AnyKey"))
  (:`Pressed`
    (`/Engine/EditorBlueprintResources/StandardMacros.FlipFlop`
      (:`A`
        (bind _returnvalue (`|CreateWidget` "/Game/Blueprints/Note_widget.Note_widget_C"))
        (`UserWidget.AddToViewport` _returnvalue 0))
      (:`B`
        (`Widget.RemoveFromParent` _returnvalue :!label _label)
        (`KismetSystemLibrary.Delay` 1.0)
        (`self.K2_DestroyActor`)
        (`/Engine/EditorBlueprintResources/StandardMacros.IncrementInt` (stale `self.ReceiveActorBeginOverlap` _output_get))))))

(event `self.ReceiveActorBeginOverlap`
  (params (OtherActor :type "Actor Object Reference"))
  (`self.EnableInput` (`GameplayStatics.GetPlayerController` 0))
  (bind _aspcmorning_star (cast `/Game/Blueprints/PCMorningStar` (`GameplayStatics.GetPlayerCharacter` 0)))
  (bind _output_get (set `/Game/Blueprints/PCMorningStar.Image Index` (`/Game/Blueprints/PCMorningStar.Image Index` _aspcmorning_star) _aspcmorning_star)))

(event `self.ReceiveActorEndOverlap`
  (params (OtherActor :type "Actor Object Reference"))
  (`self.DisableInput` null)
  (goto _label))

(fn `UserConstructionScript`)